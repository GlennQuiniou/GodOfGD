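; BP_Rune_1_Pillier is the first rune target, which unlocks its part of a chest when shot by the first-person projectile.
; On BeginPlay it finds the BP_Chest and BP_Rune_Chest_1 actors in the level, keeping the last of each.
; A projectile overlapping its box calls CERuneChest1 on the chest rune, sets the chest's Rune1 flag, then destroys the pillar rune.
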(event `self.ReceiveBeginPlay`
  (bind _outactors (`GameplayStatics.GetAllActorsOfClass` "/Game/BP_Chest.BP_Chest_C"))
  (for _array_element _outactors
    (set `self.Ref Chest` _array_element))
  (bind _outactors_2 (`GameplayStatics.GetAllActorsOfClass` "/Game/BP_Rune_Chest_1.BP_Rune_Chest_1_C"))
  (for _array_element_2 _outactors_2
    (set `self.Ref Rune 1` _array_element_2)))

(event `self.Box.OnComponentBeginOverlap`
  (params (OverlappedComponent :type "PrimitiveComponent Object Reference") (OtherActor :type "Actor Object Reference") (OtherComp :type "PrimitiveComponent Object Reference") (OtherBodyIndex :type Integer) (bFromSweep :type Boolean) (SweepResult :type "HitResult Structure (by ref)"))
  (cast `/Game/FirstPerson/Blueprints/BP_FirstPersonProjectile` OtherActor)
  (`/Game/BP_Rune_Chest_1.CE Rune Chest 1` (`self.Ref Rune 1`))
  (bind _asbp_chest (cast `/Game/BP_Chest` (`self.Ref Chest`)))
  (set `/Game/BP_Chest.Rune1` true _asbp_chest)
  (`self.K2_DestroyActor`))

(fn `UserConstructionScript`)
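; BP_Chest is a chest that stays locked until three rune flags are set, then can be opened once.
; Tick polls the flags and, when all are true, reveals a text render and clears a one-shot boolean that gates opening.
; The CEOpenChest custom event checks that gate and a second one-shot flag, hides the text and plays the LS_Chest_Sequencer level sequence.
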(event `self.ReceiveTick`
  (params (DeltaSeconds :type "Float (single-precision)"))
  (if (`self.Rune1`)
    (if (`self.Rune2`)
      (if (`self.Rune3`)
        (if (`self.UtilisationUnique`)
          (set `self.UtilisationUnique` false)
          (`SceneComponent.SetVisibility` (`self.TextRender`) true false))))))

(event `CE Open Chest`
  (if (`self.UtilisationUnique`)
    _
    (elif (`self.UtilisationUnique2`)
      (set `self.UtilisationUnique2` false)
      (`SceneComponent.SetVisibility` (`self.TextRender`) false false)
      (bind (_outactor _returnvalue) (`LevelSequencePlayer.CreateLevelSequencePlayer` "/Game/LS_Chest_Sequencer.LS_Chest_Sequencer"))
      (`MovieSceneSequencePlayer.Play` _returnvalue))))

(fn `UserConstructionScript`)